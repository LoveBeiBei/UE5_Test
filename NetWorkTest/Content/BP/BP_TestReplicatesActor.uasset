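; BP_TestReplicatesActor is a test actor for variable replication through an Armor RepNotify.
; Tick runs into a five-second Delay, then only the authority sets Armor to a random float, so the value changes roughly every five seconds.
; OnRep_Armor branches on authority to print the value with a Server or Client prefix, showing the change on each side.
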(event `self.ReceiveTick`
  (params (DeltaSeconds :type "Float (single-precision)"))
  (`KismetSystemLibrary.Delay` 5.0)
  (`/Engine/EditorBlueprintResources/ActorMacros.Switch Has Authority`
    (:`Authority`
      (set `self.Armor` (`KismetMathLibrary.RandomFloat`)))))

(fn `OnRep_Armor`
  (bind _returnvalue (`KismetStringLibrary.Conv_DoubleToString` (`self.Armor`)))
  (`/Engine/EditorBlueprintResources/ActorMacros.Switch Has Authority`
    (:`Authority`
      (`KismetSystemLibrary.PrintString` (`KismetStringLibrary.Concat_StrStr` "Server:" _returnvalue) true true (struct :`G` 0.66 :`B` 1.0 :`A` 1.0) 10.0))
    (:`Remote`
      (`KismetSystemLibrary.PrintString` (`KismetStringLibrary.Concat_StrStr` "Client:" _returnvalue) true true (struct :`G` 0.66 :`B` 1.0 :`A` 1.0) 10.0))))

(fn `UserConstructionScript`)